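; Friendly swarm bot that follows its manager's formation slot, attacks nearby enemies, overrides enemies or returns to Rael.
; Staggered looping timers drive a BotState movement switch and target acquisition, issuing AI move commands, mostly throttled by distance moved.
; Target scoring adds a TargetedByCount penalty to distance, spreading bots across enemies.
; Interpolated random jitter loosens the formation, while overriding bots register on their target when in range.
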(event EventBeginPlay
  (bind _asaicontroller (Utilities|Casting|CastToAIController (Pawn|GetController)))
  (Variables|Default|SetAIControllerRef _asaicontroller)
  (Utilities|FlowControl|Delay (Math|Random|RandomFloatinRange 0.0 0.25))
  (bind _returnvalue (Utilities|Time|SetTimerbyFunctionName 0 "UpdateFollowMovement" 0.25 true))
  (Variables|Default|SetMovementTimerHandle _returnvalue)
  (Utilities|Time|SetTimerbyFunctionName 0 "RefreshFormationJitter" (Math|Random|RandomFloatinRange 2.0 4.0))
  (Utilities|FlowControl|Delay (Math|Random|RandomFloatinRange 0.0 0.3))
  (Utilities|Time|SetTimerbyFunctionName 0 "RunTargetAcquisition" 0.3 true))

(event Collision|EventActorBeginOverlap
  (params (OtherActor :type Actor%20Object%20Reference)))

(event EventTick
  (params (DeltaSeconds :type Float%20%28single-precision%29))
  (Variables|Default|SetFormationJitter (Math|Interpolation|VInterpTo (Variables|Default|GetFormationJitter) (Variables|Default|GetTargetFormationJitter) DeltaSeconds 2.0)))

(fn ConstructionScript)

(fn UpdateFollowMovement
  (bind _owningswarmmanager (Variables|Default|GetOwningSwarmManager))
  (switch Utilities|FlowControl|Switch|SwitchonE_BotState (Variables|Default|GetBotState)
    (:NewEnumerator0
      (Utilities|IsValid _owningswarmmanager
        (:Is%20Valid
          (bind _output_get (Variables|Default|SetTargetPosition (+ (Default|GetFormationPosition _owningswarmmanager (Variables|Default|GetFormationIndex)) (Variables|Default|GetFormationJitter))))
          (Variables|Default|SetDistance (Math|Vector|Distance(Vector) (Transformation|GetActorLocation) _output_get))
          (if (not (<= (Math|Vector|Distance(Vector) (Transformation|GetActorLocation) _output_get) 8e+01))
            (if (not (< (Math|Vector|Distance(Vector) (Variables|Default|GetTargetPosition) (Variables|Default|GetLastCommandedPosition)) 1e+02))
              (Variables|/Script/Engine.CharacterMovementComponent|SetMaxWalkSpeed (Variables|Character|GetCharacterMovement) (* (Math|Float|Clamp(Float) (Math|Float|SafeDivide (Variables|Default|GetDistance) 3e+02) 0.3) (Variables|Default|GetBaseMaxSpeed)))
              (AI|Navigation|MovetoLocation (Variables|Default|GetAIControllerRef) (Variables|Default|GetTargetPosition) 5e+01 true true false true 0))))))
    (:NewEnumerator1
      (if (Utilities|IsValid (Variables|Default|GetCurrentTarget))
        (bind _asbp_enemy_base (Utilities|Casting|CastToBP_EnemyBase (Variables|Default|GetCurrentTarget)))
        (if (> (Variables|/Game/BadSignalContent/Blueprints/Bots/BP_EnemyBase.BP_EnemyBase_C|GetHealth _asbp_enemy_base) 0.0)
          (bind _output_get_2 (LocalVariables|SetDistToTarget (Math|Vector|Distance(Vector) (Transformation|GetActorLocation (Variables|Default|GetCurrentTarget)) (Transformation|GetActorLocation))))
          (if (> _output_get_2 (Variables|Default|GetAggroRange))
            ;[0.15 0.15 0.15 0.5] reduce targeted by count
            (if (Utilities|IsValid (Variables|Default|GetCurrentTarget)) :!label _label
              (bind _asbp_enemy_base_2 (Utilities|Casting|CastToBP_EnemyBase (Variables|Default|GetCurrentTarget)))
              (Variables|/Game/BadSignalContent/Blueprints/Bots/BP_EnemyBase.BP_EnemyBase_C|SetTargetedByCount _asbp_enemy_base_2 (Math|Integer|Clamp(Integer) (- (Variables|/Game/BadSignalContent/Blueprints/Bots/BP_EnemyBase.BP_EnemyBase_C|GetTargetedByCount _asbp_enemy_base_2) 1) 0 999)))
            (Variables|Default|SetCurrentTarget 0)
            (Variables|Default|SetBotState "NewEnumerator0")
            (Variables|Default|SetLastChaseCommandPosition "0, 0, 0")
            (else
              ;[0.15 0.15 0.15 0.5] chase AND attack at once
              (if (not (< (Math|Vector|Distance(Vector) (Variables|Default|GetLastChaseCommandPosition) (Transformation|GetActorLocation (Variables|Default|GetCurrentTarget))) 4e+01))
                (AI|Navigation|MovetoLocation (Variables|Default|GetAIControllerRef) (Transformation|GetActorLocation (Variables|Default|GetCurrentTarget)) 1e+01 true true false true 0)
                (Variables|Default|SetLastChaseCommandPosition (Transformation|GetActorLocation (Variables|Default|GetCurrentTarget)))
                (if (<= (Math|Vector|Distance(Vector) (Variables|Default|GetLastChaseCommandPosition) (Transformation|GetActorLocation (Variables|Default|GetCurrentTarget))) (Variables|Default|GetAttackRange))
                  (if (Variables|Default|GetbCanAttack)
                    (bind _asbp_enemy_base_3 (Utilities|Casting|CastToBP_EnemyBase (Variables|Default|GetCurrentTarget)))
                    (Default|ReceiveBotDamage _asbp_enemy_base_3 (Variables|Default|GetAttackDamage))
                    (Variables|Default|SetbCanAttack false)
                    (Utilities|Time|SetTimerbyFunctionName 0 "ResetAttack" (Variables|Default|GetAttackCooldown)))))))
          (else
            (goto _label)))
        (else
          (goto _label))))
    (:NewEnumerator2
      (CallFunction|UpdateOverrideMovement))
    (:NewEnumerator3
      (bind _output_get_3 (Variables|Default|SetRaelPosition (Transformation|GetActorLocation (Variables|/Game/BadSignalContent/Blueprints/Player/BP_SwarmManager.BP_SwarmManager_C|GetRaelRef (Variables|Default|GetOwningSwarmManager)))))
      (if (<= (Math|Vector|Distance(Vector) (Transformation|GetActorLocation) _output_get_3) 2.5e+02)
        ;[0.15 0.15 0.15 0.5] reached
        (Variables|/Script/Engine.CharacterMovementComponent|SetMaxWalkSpeed (Variables|Character|GetCharacterMovement) (Variables|Default|GetBaseMaxSpeed))
        (Variables|Default|SetLastCommandedPosition "0, 0, 0")
        (Variables|Default|SetBotState "NewEnumerator0")
        (elif (not (< (Math|Vector|Distance(Vector) (Variables|Default|GetRaelPosition) (Variables|Default|GetLastCommandedPosition)) 25.0))
          (AI|Navigation|MovetoLocation (Variables|Default|GetAIControllerRef) (Variables|Default|GetRaelPosition) 7e+01 true true false true 0)
          (Variables|Default|SetLastCommandedPosition (Variables|Default|GetRaelPosition)))))))

(fn RefreshFormationJitter
  (Variables|Default|SetTargetFormationJitter (Math|Vector|MakeVector (Math|Random|RandomFloatinRange -2e+01 2e+01) (Math|Random|RandomFloatinRange -2e+01 2e+01) 0.0))
  (Utilities|Time|SetTimerbyFunctionName 0 "RefreshFormationJitter" (Math|Random|RandomFloatinRange 2.0 4.0)))

(fn FindBestTarget
  (bind _outactors (Actor|GetAllActorswithTag "Enemy"))
  (for _array_element _outactors
    (if (Utilities|IsValid _array_element)
      (bind _output_get (LocalVariables|SetDistToEnemy (Math|Vector|Distance(Vector) (Transformation|GetActorLocation _array_element) (Transformation|GetActorLocation))))
      (if (not (> _output_get (Variables|Default|GetAggroRange)))
        (bind _asbp_enemy_base (Utilities|Casting|CastToBP_EnemyBase _array_element))
        (if (< (+ (LocalVariables|GetDistToEnemy) (* (Variables|/Game/BadSignalContent/Blueprints/Bots/BP_EnemyBase.BP_EnemyBase_C|GetTargetedByCount _asbp_enemy_base) 200)) (LocalVariables|GetBestScore))
          (LocalVariables|SetBestScore (+ (LocalVariables|GetDistToEnemy) (* (Variables|/Game/BadSignalContent/Blueprints/Bots/BP_EnemyBase.BP_EnemyBase_C|GetTargetedByCount _asbp_enemy_base) 200)))
          (LocalVariables|SetBestEnemy _array_element)))))
  (return (LocalVariables|GetBestEnemy)))

(fn RunTargetAcquisition
  (if (Utilities|Enum|Equal(Enum) (Variables|Default|GetBotState) "NewEnumerator0")
    (bind _besttarget (CallFunction|FindBestTarget))
    (bind _output_get (LocalVariables|SetFoundTarget _besttarget))
    (if (Utilities|IsValid _output_get)
      (Variables|Default|SetCurrentTarget (LocalVariables|GetFoundTarget))
      (bind _asbp_enemy_base (Utilities|Casting|CastToBP_EnemyBase (LocalVariables|GetFoundTarget)))
      (bind _result (Math|Integer|IncrementInt (Variables|/Game/BadSignalContent/Blueprints/Bots/BP_EnemyBase.BP_EnemyBase_C|GetTargetedByCount _asbp_enemy_base))
        (:%20%20
          (Variables|/Game/BadSignalContent/Blueprints/Bots/BP_EnemyBase.BP_EnemyBase_C|SetTargetedByCount _asbp_enemy_base _result)
          (Variables|Default|SetBotState "NewEnumerator1")
          (Variables|Default|SetbCanAttack false)
          (Utilities|Time|SetTimerbyFunctionName 0 "ResetAttack" (Math|Random|RandomFloatinRange 0.0 0.2) true))))))

(fn ResetAttack
  (Variables|Default|SetbCanAttack true))

(fn UpdateOverrideMovement
  (bind _self self)
  (bind _self_2 self)
  (if (Utilities|IsValid (Variables|Default|GetOverrideTarget))
    (if (> (Math|Vector|Distance(Vector) (Transformation|GetActorLocation) (Transformation|GetActorLocation (Variables|Default|GetOverrideTarget))) (Variables|Default|GetOverrideRange))
      (AI|Navigation|MovetoLocation (Variables|Default|GetAIControllerRef) (Transformation|GetActorLocation (Variables|Default|GetOverrideTarget)) -1.0 true true false true 0)
      (if (not (== (Utilities|Array|FindItem (Variables|/Game/BadSignalContent/Blueprints/Bots/BP_EnemyBase.BP_EnemyBase_C|GetOverridingBots (Variables|Default|GetOverrideTarget)) _self_2) -1))
        (Utilities|Array|RemoveItem (Variables|/Game/BadSignalContent/Blueprints/Bots/BP_EnemyBase.BP_EnemyBase_C|GetOverridingBots (Variables|Default|GetOverrideTarget)) _self_2))
      (elif (== (Utilities|Array|FindItem (Variables|/Game/BadSignalContent/Blueprints/Bots/BP_EnemyBase.BP_EnemyBase_C|GetOverridingBots (Variables|Default|GetOverrideTarget)) _self) -1)
        (Utilities|Array|Add (Variables|/Game/BadSignalContent/Blueprints/Bots/BP_EnemyBase.BP_EnemyBase_C|GetOverridingBots (Variables|Default|GetOverrideTarget)) _self)))
    (else
      (bind _besttarget (CallFunction|FindBestTarget))
      (if (Utilities|IsValid _besttarget)
        (bind _asbp_enemy_base (Utilities|Casting|CastToBP_EnemyBase _besttarget))
        (Variables|Default|SetOverrideTarget _asbp_enemy_base)
        (else
          (Variables|Default|SetBotState "NewEnumerator0"))))))

(fn TakeDamage
  (params (DamageAmount :type Float%20%28double-precision%29))
  (bind _self self)
  (bind _overridetarget (Variables|Default|GetOverrideTarget))
  (bind _overridingbots (Variables|/Game/BadSignalContent/Blueprints/Bots/BP_EnemyBase.BP_EnemyBase_C|GetOverridingBots _overridetarget))
  (bind _returnvalue (Utilities|Array|FindItem _overridingbots _self))
  (bind _output_get (Variables|Default|SetHealth (- (Variables|Default|GetHealth) DamageAmount)))
  (if (<= _output_get 0.0)
    (if (Utilities|Enum|Equal(Enum) (Variables|Default|GetBotState) "NewEnumerator2")
      (if (Utilities|IsValid _overridetarget)
        (if (not (== _returnvalue -1))
          (Utilities|Array|RemoveIndex _overridingbots _returnvalue))
        (else
          (Default|UnregisterBot (Variables|Default|GetOwningSwarmManager) self)
          (Actor|DestroyActor))))))