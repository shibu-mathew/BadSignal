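; Swarm manager that tracks the player's bots and keeps their formation around a movable leash point.
; Each Tick it eases an offset toward a desired offset and adds it to the owner's location to place the leash point.
; Registered bots get formation indices on a ring that widens with swarm size.
; Recall resets steering, releases enemy targeting counts and speeds up the bots.
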(event EventBeginPlay
  (bind _asbp_rael (Utilities|Casting|CastToBP_Rael (Game|GetPlayerCharacter 0)))
  (Variables|Default|SetRaelRef _asbp_rael))

(event EventTick
  (params (DeltaSeconds :type Float%20%28single-precision%29))
  (CallFunction|UpdateLeashPoint DeltaSeconds))

(fn RegisterBot
  (params (Bot :type BP%20Friendly%20Bot%20Object%20Reference))
  (bind _swarmbots (Variables|Default|GetSwarmBots))
  (bind _returnvalue (Utilities|Array|Add _swarmbots Bot))
  (Variables|/Game/BadSignalContent/Blueprints/Bots/BP_FriendlyBot.BP_FriendlyBot_C|SetFormationIndex Bot _returnvalue)
  (Variables|/Game/BadSignalContent/Blueprints/Bots/BP_FriendlyBot.BP_FriendlyBot_C|SetOwningSwarmManager Bot self)
  (Default|CallOnBotRegistered Bot)
  (Default|CallOnSwarmSizeChanged (Utilities|Array|Length _swarmbots)))

(fn UnregisterBot
  (params (Bot :type BP%20Friendly%20Bot%20Object%20Reference))
  (bind _swarmbots (Variables|Default|GetSwarmBots))
  (Utilities|Array|RemoveItem _swarmbots Bot)
  (for (_array_element _array_index) _swarmbots
    (Variables|/Game/BadSignalContent/Blueprints/Bots/BP_FriendlyBot.BP_FriendlyBot_C|SetFormationIndex _array_element _array_index)
    (Default|CallOnBotLost Bot)
    (Default|CallOnSwarmSizeChanged (Utilities|Array|Length _swarmbots))))

(fn GetFormationPosition
  (params (Index :type Integer))
  (bind _returnvalue (Math|Conversions|ToFloat(Integer) Index))
  (bind _swarmbots (Variables|Default|GetSwarmBots))
  (bind _returnvalue_2 (Utilities|Array|Length _swarmbots))
  (bind _returnvalue_3 (Math|Conversions|ToFloat(Integer) _returnvalue_2))
  (bind _returnvalue_4 (Math|Float|SafeDivide _returnvalue _returnvalue_3))
  (bind _returnvalue_5 (* _returnvalue_4 360))
  (return (+ (Variables|Default|GetLeashPoint) (* (Math|Vector|MakeVector (Math|Trig|Cos(Degrees) _returnvalue_5) (Math|Trig|Sin(Degrees) _returnvalue_5) 0.0) (+ (* _returnvalue_2 8) (Variables|Default|GetFormationRadius))))))

(fn UpdateLeashPoint
  (params (DeltaTime :type Float%20%28double-precision%29))
  (bind _output_get (Variables|Default|SetSwarmTargetOffset (Math|Interpolation|VInterpTo (Variables|Default|GetSwarmTargetOffset) (Variables|Default|GetDesiredOffset) DeltaTime (Variables|Default|GetSwarmSpeed))))
  (Variables|Default|SetLeashPoint (+ _output_get (Transformation|GetActorLocation (Components|GetOwner)))))

(fn RecallAllBots
  (Variables|Default|SetSwarmTargetOffset "0, 0, 0")
  (Variables|Default|SetDesiredOffset "0, 0, 0")
  (Variables|Default|SetbIsSteering false)
  (for _array_element (Variables|Default|GetSwarmBots)
    (if (Utilities|IsValid _array_element)
      (Variables|/Game/BadSignalContent/Blueprints/Bots/BP_FriendlyBot.BP_FriendlyBot_C|SetBotState _array_element "NewEnumerator3")
      (if (Utilities|IsValid (Variables|/Game/BadSignalContent/Blueprints/Bots/BP_FriendlyBot.BP_FriendlyBot_C|GetCurrentTarget _array_element))
        (bind _asbp_enemy_base (Utilities|Casting|CastToBP_EnemyBase (Variables|/Game/BadSignalContent/Blueprints/Bots/BP_FriendlyBot.BP_FriendlyBot_C|GetCurrentTarget _array_element)))
        (Variables|/Game/BadSignalContent/Blueprints/Bots/BP_EnemyBase.BP_EnemyBase_C|SetTargetedByCount _asbp_enemy_base (Math|Integer|Clamp(Integer) (- (Variables|/Game/BadSignalContent/Blueprints/Bots/BP_EnemyBase.BP_EnemyBase_C|GetTargetedByCount _asbp_enemy_base) 1) 0 999)))
      (Variables|/Game/BadSignalContent/Blueprints/Bots/BP_FriendlyBot.BP_FriendlyBot_C|SetCurrentTarget _array_element 0)
      (Variables|/Script/Engine.CharacterMovementComponent|SetMaxWalkSpeed (Variables|/Script/Engine.Character|GetCharacterMovement _array_element) (* (Variables|/Game/BadSignalContent/Blueprints/Bots/BP_FriendlyBot.BP_FriendlyBot_C|GetBaseMaxSpeed _array_element) 1.5))
      (Variables|/Game/BadSignalContent/Blueprints/Bots/BP_FriendlyBot.BP_FriendlyBot_C|SetLastCommandedPosition _array_element "0, 0, 0"))))