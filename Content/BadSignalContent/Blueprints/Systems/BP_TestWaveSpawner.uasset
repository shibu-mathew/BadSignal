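; Test wave spawner that periodically spawns civilian and jammer enemies around the level's TargetPoints, up to a cap on living enemies.
; A looping timer runs SpawnWave, placing civilians first, then jammers, at random points with XY jitter; kill-event bindings track the live count.
; Waves count only when civilians leave room under the cap.
; Civilians per wave grow every third wave; jammers every fifteenth, as that check is nested.
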(event Custom|OnAnyEnemyKilled
  (params (KilledEnemy :type BP%20Enemy%20Base%20Object%20Reference))
  (Variables|Default|SetCurrentEnemyCount (Math|Integer|Clamp(Integer) (- (Variables|Default|GetCurrentEnemyCount) 1) 0 999)))

(event EventBeginPlay
  (bind _spawnpoints (Variables|Default|GetSpawnPoints))
  (bind _outactors (Actor|GetAllActorsOfClass "/Script/Engine.TargetPoint"))
  (for _array_element _outactors
    (Utilities|Array|Add _spawnpoints (Transformation|GetActorLocation _array_element)))
  (if (> (Utilities|Array|Length _spawnpoints) 0)
    (Utilities|Time|SetTimerbyFunctionName 0 "SpawnWave" (Variables|Default|GetSpawnInterval) true)
    (else
      (Development|PrintString "NO SPAWN POINTS FOUND"))))

(event Collision|EventActorBeginOverlap
  (params (OtherActor :type Actor%20Object%20Reference)))

(event EventTick
  (params (DeltaSeconds :type Float%20%28single-precision%29)))

(fn ConstructionScript)

(fn SpawnWave
  (bind _spawnpoints (Variables|Default|GetSpawnPoints))
  (bind _spawnpoints_2 (Variables|Default|GetSpawnPoints))
  (if (not (>= (Variables|Default|GetCurrentEnemyCount) (Variables|Default|GetMaxEnemiesAlive)))
    (Utilities|FlowControl|ForLoopwithBreak 0 (- (Variables|Default|GetCiviliansPerWave) 1) :!label _label
      (:LoopBody
        (bind _returnvalue (Game|SpawnActorfromClass "/Game/BadSignalContent/Blueprints/Bots/BP_EnemyCivilian.BP_EnemyCivilian_C" (Math|Transform|MakeTransform (+ (Math|Vector|MakeVector (Math|Random|RandomFloatinRange -2e+02 2e+02) (Math|Random|RandomFloatinRange -2e+02 2e+02) 0.0) (Utilities|Array|Get(acopy) _spawnpoints (Math|Random|RandomIntegerinRange 0 (- (Utilities|Array|Length _spawnpoints) 1))))) "AlwaysSpawn" "MultiplyWithRoot" 0 0))
        (EventDispatchers|BindEventtoOnEnemyKilled _returnvalue (EventDispatchers|CreateEvent :!event Custom|OnAnyEnemyKilled))
        (bind _output_get (Variables|Default|SetCurrentEnemyCount (+ (Variables|Default|GetCurrentEnemyCount) 1)))
        (if (>= _output_get (Variables|Default|GetMaxEnemiesAlive))
          (goto _label Break)))
      (:Completed
        (if (not (>= (Variables|Default|GetCurrentEnemyCount) (Variables|Default|GetMaxEnemiesAlive)))
          (Utilities|FlowControl|ForLoopwithBreak 0 (- (Variables|Default|GetJammersPerWave) 1) :!label _label_2
            (:LoopBody
              (bind _returnvalue_2 (Game|SpawnActorfromClass "/Game/BadSignalContent/Blueprints/Bots/BP_EnemyJammer.BP_EnemyJammer_C" (Math|Transform|MakeTransform (+ (Math|Vector|MakeVector (Math|Random|RandomFloatinRange -2e+02 2e+02) (Math|Random|RandomFloatinRange -2e+02 2e+02) 0.0) (Utilities|Array|Get(acopy) _spawnpoints_2 (Math|Random|RandomIntegerinRange 0 (- (Utilities|Array|Length _spawnpoints_2) 1))))) "Undefined" "MultiplyWithRoot" 0 0))
              (EventDispatchers|BindEventtoOnEnemyKilled _returnvalue_2 (EventDispatchers|CreateEvent :!event Custom|OnAnyEnemyKilled))
              (bind _output_get_2 (Variables|Default|SetCurrentEnemyCount (+ (Variables|Default|GetCurrentEnemyCount) 1)))
              (if (>= _output_get_2 (Variables|Default|GetMaxEnemiesAlive))
                (goto _label_2 Break)))
            (:Completed
              (bind _output_get_3 (Variables|Default|SetWaveCount (+ (Variables|Default|GetWaveCount) 1)))
              (if (== (Math|Integer|%(Integer) _output_get_3 3) 0)
                (Variables|Default|SetCiviliansPerWave (+ (Variables|Default|GetCiviliansPerWave) 1))
                (if (== (Math|Integer|%(Integer) _output_get_3 5) 0)
                  (Variables|Default|SetJammersPerWave (+ (Variables|Default|GetJammersPerWave) 1)))))))))))