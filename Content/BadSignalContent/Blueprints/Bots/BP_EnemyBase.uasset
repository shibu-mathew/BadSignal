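; Base enemy Blueprint that detects the player character Rael, chases it and deals damage in attack range, and is destroyed when bot damage drains its health.
; An enum state moves from Idle to Pursuing to Attacking, with looping timers instead of Tick; the detection timer hands off to a pursue timer.
; Pursuit reissues AI MoveTo only after Rael moves far enough, and attacks use a timed cooldown.
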(event EventBeginPlay
  (bind _asbp_rael (Utilities|Casting|CastToBP_Rael (Game|GetPlayerCharacter 0)))
  (Variables|Default|SetRaelRef _asbp_rael)
  (bind _asaicontroller (Utilities|Casting|CastToAIController (Pawn|GetController)))
  (Variables|Default|SetAIControllerRef _asaicontroller)
  (Variables|/Script/Engine.CharacterMovementComponent|SetMaxWalkSpeed (Variables|Character|GetCharacterMovement) (Variables|Default|GetMoveSpeed))
  (bind _returnvalue (Utilities|Time|SetTimerbyFunctionName 0 "RunDetection" 0.5 true))
  (Variables|Default|SetDetectionTimerHandle _returnvalue))

(fn ConstructionScript)

(fn ReceiveBotDamage
  (params (DamageAmount :type Float%20%28double-precision%29))
  (bind _output_get (Variables|Default|SetHealth (- (Variables|Default|GetHealth) DamageAmount)))
  (if (<= _output_get 0.0)
    (Variables|Default|SetTargetedByCount 0)
    (Actor|DestroyActor)))

(fn RunDetection
  (if (Utilities|Enum|Equal(Enum) (Variables|Default|GetEnemyState) "NewEnumerator0")
    (if (<= (Math|Vector|Distance(Vector) (Transformation|GetActorLocation (Variables|Default|GetRaelRef)) (Transformation|GetActorLocation)) (Variables|Default|GetDetectionRange))
      (Variables|Default|SetEnemyState "NewEnumerator1")
      (Utilities|Time|ClearandInvalidateTimerbyHandle (Variables|Default|GetDetectionTimerHandle))
      (bind _returnvalue (Utilities|Time|SetTimerbyFunctionName 0 "UpdatePursue" 0.4 true))
      (Variables|Default|SetPursueTimerHandle _returnvalue))))

(fn UpdatePursue
  (bind _raelref (Variables|Default|GetRaelRef))
  (bind _raelref_2 (Variables|Default|GetRaelRef))
  (bind _returnvalue (Transformation|GetActorLocation _raelref_2))
  (switch Utilities|FlowControl|Switch|SwitchonE_EnemyState (Variables|Default|GetEnemyState)
    (:NewEnumerator1
      (if (Utilities|IsValid _raelref)
        (if (<= (Math|Vector|Distance(Vector) (Transformation|GetActorLocation) (Transformation|GetActorLocation _raelref)) (Variables|Default|GetAttackRange))
          (AI|Navigation|StopMovement (Variables|Default|GetAIControllerRef))
          (Variables|Default|SetEnemyState "NewEnumerator2")
          (elif (not (< (Math|Vector|Distance(Vector) (Transformation|GetActorLocation (Variables|Default|GetRaelRef)) (Variables|Default|GetLastPursueCommandPos)) 8e+01))
            (AI|Navigation|MovetoLocation (Variables|Default|GetAIControllerRef) _returnvalue (* (Variables|Default|GetAttackRange) 0.8) true true false true 0)
            (Variables|Default|SetLastPursueCommandPos _returnvalue)))))
    (:NewEnumerator2
      (if (> (Math|Vector|Distance(Vector) (Transformation|GetActorLocation (Variables|Default|GetRaelRef)) (Transformation|GetActorLocation)) (Variables|Default|GetAttackRange))
        (Variables|Default|SetEnemyState "NewEnumerator1")
        (Variables|Default|SetLastPursueCommandPos "0, 0, 0")
        (elif (Variables|Default|GetbCanAttack)
          (Default|RecieveDamage (Variables|Default|GetRaelRef) (Variables|Default|GetAttackDamage))
          (Variables|Default|SetbCanAttack false)
          (Utilities|Time|SetTimerbyFunctionName 0 "ResetEnemyAttack" 0.5))))))

(fn ResetEnemyAttack
  (Variables|Default|SetbCanAttack true))